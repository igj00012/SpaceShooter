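; Boss enemy for the SpaceShooter game, a tougher child of an enemy base class with high life, a point reward and a slow entrance.
; BeginPlay overrides inherited stats, then after a short delay stops movement and enables shooting.
; Move calls the parent only while Moving is set.
; Fire spawns lasers from three fire points aligned to the boss's rotation, then clears ReadyToShoot.
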(event `self.ReceiveBeginPlay`
  (`parent.ReceiveBeginPlay`)
  (set `self.Lifes` 70.0)
  (set `self.Points` 15)
  (set `self.MovementVector` (`self.GetActorForwardVector`))
  (set `self.Speed` 25.0)
  (set `self.DestroyOnWall` false)
  (set `self.DelayShoot` 7.0)
  (`KismetSystemLibrary.Delay` 3.0)
  (set `self.Moving` false)
  (set `self.ReadyToShoot` true))

(event `self.ReceiveTick`
  (params (DeltaSeconds :type "Float (single-precision)"))
  (`parent.ReceiveTick` DeltaSeconds))

(fn `Fire`
  (bind _returnvalue (`|SpawnActorFromClass` (`self.Laser`) (`SceneComponent.K2_GetComponentToWorld` (`self.FirePoint`)) "Undefined" "MultiplyWithRoot" null null))
  (`self.K2_SetActorRotation` _returnvalue (`self.K2_GetActorRotation`) false)
  (bind _returnvalue_2 (`|SpawnActorFromClass` (`self.Laser`) (`SceneComponent.K2_GetComponentToWorld` (`self.FirePoint1`)) "Undefined" "MultiplyWithRoot" null null))
  (`self.K2_SetActorRotation` _returnvalue_2 (`self.K2_GetActorRotation`) false)
  (bind _returnvalue_3 (`|SpawnActorFromClass` (`self.Laser`) (`SceneComponent.K2_GetComponentToWorld` (`self.FirePoint2`)) "Undefined" "MultiplyWithRoot" null null))
  (`self.K2_SetActorRotation` _returnvalue_3 (`self.K2_GetActorRotation`) false)
  (set `self.ReadyToShoot` false))

(fn `Move`
  (params (Detla_Time :type "Float (double-precision)"))
  (if (`self.Moving`)
    (`parent.Move` Detla_Time)))

(fn `UserConstructionScript`
  (`parent.UserConstructionScript`))