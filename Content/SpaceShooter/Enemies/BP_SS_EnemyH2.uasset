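; BP_SS_EnemyH2 is a space shooter enemy child Blueprint that moves sideways and fires two shots at once, worth 7 points.
; On overlapping an actor tagged "Pared" (wall), it steps along negative X, flips its MovementVector and shortens DelayShoot, so each bounce tightens the shot delay.
; Fire spawns Ammo at two fire points, aligned to the enemy's rotation.
; Movement and fire timing are not in this graph.
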(event `self.ReceiveBeginPlay`
  (`parent.ReceiveBeginPlay`)
  (set `self.Points` 7)
  (set `self.MovementVector` (`self.GetActorRightVector`))
  (set `self.IsRight` true))

(event `self.ReceiveActorBeginOverlap`
  (params (OtherActor :type "Actor Object Reference"))
  (bind _returnvalue (`self.GetActorRightVector`))
  (`parent.ReceiveActorBeginOverlap` OtherActor)
  (if (`KismetArrayLibrary.Array_Contains` (`Actor.Tags` OtherActor) "Pared")
    (`self.K2_SetActorLocation` (- (`self.K2_GetActorLocation`) (15.0 0.0 0.0)))
    (if (`self.IsRight`)
      (set `self.IsRight` false)
      (set `self.MovementVector` (* _returnvalue -1.0))
      (else
        (set `self.IsRight` true)
        (set `self.MovementVector` _returnvalue)))
    (set `self.DelayShoot` (- (`self.DelayShoot`) 0.1))))

(fn `Fire`
  (bind _returnvalue (`|SpawnActorFromClass` (`self.Ammo`) (`SceneComponent.K2_GetComponentToWorld` (`self.FirePoint`)) "Undefined" "MultiplyWithRoot" null null))
  (`self.K2_SetActorRotation` _returnvalue (`self.K2_GetActorRotation`) false)
  (bind _returnvalue_2 (`|SpawnActorFromClass` (`self.Ammo`) (`SceneComponent.K2_GetComponentToWorld` (`self.FirePoint1`)) "Undefined" "MultiplyWithRoot" null null))
  (`self.K2_SetActorRotation` _returnvalue_2 (`self.K2_GetActorRotation`) false))

(fn `UserConstructionScript`
  (`parent.UserConstructionScript`))