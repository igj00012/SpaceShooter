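; Enemy laser actor for the space shooter that expires after LifeTime and shows hit effects on pawns it touches.
; Begin overlap stores any Pawn as Player and sets an Overlapping flag, which end overlap clears for that same actor.
; While the flag is set, Tick spawns an explosion emitter at that pawn and plays a 2D sound every frame, without applying damage.
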(event `self.ReceiveBeginPlay`
  (`self.SetLifeSpan` (`self.LifeTime`)))

(event `self.ReceiveActorBeginOverlap`
  (params (OtherActor :type "Actor Object Reference"))
  (bind _aspawn (cast `Pawn` OtherActor))
  (set `self.Player` _aspawn)
  (set `self.Overlapping` true))

(event `self.ReceiveTick`
  (params (DeltaSeconds :type "Float (single-precision)"))
  (if (`self.Overlapping`)
    (`GameplayStatics.SpawnEmitterAtLocation` "/Game/StarterContent/Particles/P_Explosion.P_Explosion" (`self.K2_GetActorLocation` (`self.Player`)))
    (`GameplayStatics.PlaySound2D` "/Game/StarterContent/Audio/Explosion02.Explosion02" 1.0 1.0 0.0 null null)))

(event `self.ReceiveActorEndOverlap`
  (params (OtherActor :type "Actor Object Reference"))
  (if (== OtherActor (`self.Player`))
    (set `self.Overlapping` false)))

(fn `UserConstructionScript`)