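; BP_SS_EnemyH is a space shooter enemy that moves sideways, bouncing between walls.
; BeginPlay overrides inherited settings for direction, points and lives, and turns off destruction on wall contact.
; Overlapping an actor tagged "Pared" flips the movement vector along the actor's right axis.
; Each flip from right to left also shortens the shoot delay, with no lower limit here.
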(event `self.ReceiveBeginPlay`
  (`parent.ReceiveBeginPlay`)
  (set `self.MovementVector` (`self.GetActorRightVector`))
  (set `self.IsRight` true)
  (set `self.Points` 3)
  (set `self.Lifes` 15.0)
  (set `self.DestroyOnWall` false))

(event `self.ReceiveActorBeginOverlap`
  (params (OtherActor :type "Actor Object Reference"))
  (bind _returnvalue (`self.GetActorRightVector`))
  (`parent.ReceiveActorBeginOverlap` OtherActor)
  (if (`KismetArrayLibrary.Array_Contains` (`Actor.Tags` OtherActor) "Pared")
    (if (`self.IsRight`)
      (set `self.IsRight` false)
      (set `self.MovementVector` (* _returnvalue -1.0))
      (set `self.DelayShoot` (- (`self.DelayShoot`) 0.1))
      (else
        (set `self.IsRight` true)
        (set `self.MovementVector` _returnvalue)))))

(fn `UserConstructionScript`
  (`parent.UserConstructionScript`))