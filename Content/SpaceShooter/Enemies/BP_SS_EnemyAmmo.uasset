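; Enemy projectile Blueprint for the space shooter that flies straight ahead and destroys itself on relevant overlaps.
; Tick moves it along its forward vector at Speed, scaled by delta time and without sweep.
; Overlapping any Pawn spawns an explosion effect and sound, then destroys it after a short delay; no damage is applied here.
; Overlapping actors tagged as wall ("Pared") or player ammo destroys it immediately.
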(event `self.ReceiveActorBeginOverlap`
  (params (OtherActor :type "Actor Object Reference"))
  (bind _tags (`Actor.Tags` OtherActor))
  (cast `Pawn` OtherActor
    (:`then`
      ; Overlap with player
      (`GameplayStatics.SpawnEmitterAtLocation` "/Game/StarterContent/Particles/P_Explosion.P_Explosion" (`self.K2_GetActorLocation`))
      (`GameplayStatics.PlaySound2D` "/Game/StarterContent/Audio/Explosion01.Explosion01" 1.0 1.0 0.0 null null)
      (`KismetSystemLibrary.Delay` 0.2)
      (`self.K2_DestroyActor`))
    (:`CastFailed`
      ; Overlap with wall
      (if (`KismetArrayLibrary.Array_Contains` _tags "Pared")
        (`self.K2_DestroyActor`)
        (else
          ; Overlap with player ammo
          (if (`KismetArrayLibrary.Array_Contains` _tags "PlayerAmmo")
            (`self.K2_DestroyActor`)))))))

(event `self.ReceiveTick`
  (params (DeltaSeconds :type "Float (single-precision)"))
  ; Enemy ammo movement logic
  (`self.K2_SetActorLocation` (+ (* (`self.GetActorForwardVector`) (* DeltaSeconds (`self.Speed`))) (`self.K2_GetActorLocation`))))

(fn `UserConstructionScript`)