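; Base enemy actor for the space shooter that flies along its initial forward vector and periodically fires Ammo from FirePoint.
; Tick drives movement and the shot timer, with a delay before shooting is first enabled.
; Overlaps with Player-tagged actors remove a life, and at zero report Points to SS_GameMode.
; Zero lives, or Pared-tagged walls when DestroyOnWall is set, trigger the OnEnemyDestroy dispatcher, whose bound event destroys the actor shortly after.
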(event `self.ReceiveBeginPlay`
  (set `self.MovementVector` (`self.GetActorForwardVector`))
  (add `self.OnEnemyDestroy` (delegate `Destroyed_Event`)))

(event `Destroyed_Event`
  (`KismetSystemLibrary.Delay` 0.2)
  (`self.K2_DestroyActor`))

(event `self.ReceiveActorBeginOverlap`
  (params (OtherActor :type "Actor Object Reference"))
  (bind _tags (`Actor.Tags` OtherActor))
  ; Overlap with player
  (if (`KismetArrayLibrary.Array_Contains` _tags "Player")
    (`self.UpdateLifes`)
    (if (== (`self.Lifes`) 0)
      (`self.OnEnemyDestroy`)
      (bind _asss_game_mode (cast `/Game/SpaceShooter/SS_GameMode` (`GameplayStatics.GetGameMode`)))
      (`/Game/SpaceShooter/SS_GameMode.Enemy_Destroyed` _asss_game_mode (`self.Points`)))
    (else
      ; Overlap with wall
      (if (`KismetArrayLibrary.Array_Contains` _tags "Pared")
        (if (`self.DestroyOnWall`)
          (`self.OnEnemyDestroy`))))))

(event `UpdateLifes`
  (bind _lifes (`self.Lifes`))
  ; Update lifes logic
  (if (> _lifes 0)
    (set `self.Lifes` (- _lifes 1))))

(event `self.ReceiveTick`
  (params (DeltaSeconds :type "Float (single-precision)"))
  (`self.Move` DeltaSeconds)
  (bind _output_get (set `self.ShotCurrentTime` (+ DeltaSeconds (`self.ShotCurrentTime`))))
  (if (> _output_get (`self.DelayShoot`))
    (set `self.ShotCurrentTime` 0.0)
    (if (`self.ReadyToShoot`)
      (`self.Fire`)
      (else
        (`KismetSystemLibrary.Delay` (`self.DelayShoot`))
        (set `self.ReadyToShoot` true)))))

(fn `Fire`
  (bind _returnvalue (`|SpawnActorFromClass` (`self.Ammo`) (`SceneComponent.K2_GetComponentToWorld` (`self.FirePoint`)) "Undefined" "MultiplyWithRoot" null null))
  (`self.K2_SetActorRotation` _returnvalue (`self.K2_GetActorRotation`) false))

(fn `Move`
  (params (Detla_Time :type "Float (double-precision)"))
  (`self.K2_SetActorLocation` (+ (`self.K2_GetActorLocation`) (* (* Detla_Time (`self.Speed`)) (`self.MovementVector`)))))

(fn `UserConstructionScript`)