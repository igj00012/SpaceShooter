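; BP_SS_EnemyL is an enemy variant in the space shooter that stays in place, with a high life count and a laser attack.
; BeginPlay calls the parent, then overrides its stats: points, shot delay, lives, a zero movement vector and no destruction on walls.
; Fire spawns a Laser at FirePoint, aligns it to the enemy's rotation, clears ReadyToShoot and plays the laser sound.
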(event `self.ReceiveBeginPlay`
  (`parent.ReceiveBeginPlay`)
  (set `self.Points` 7)
  (set `self.DelayShoot` 4.0)
  (set `self.MovementVector` (0.0 0.0 0.0))
  (set `self.Lifes` 40.0)
  (set `self.DestroyOnWall` false))

(fn `Fire`
  (bind _returnvalue (`|SpawnActorFromClass` (`self.Laser`) (`SceneComponent.K2_GetComponentToWorld` (`self.FirePoint`)) "Undefined" "MultiplyWithRoot" null null))
  (`self.K2_SetActorRotation` _returnvalue (`self.K2_GetActorRotation`) false)
  (set `self.ReadyToShoot` false)
  (`GameplayStatics.PlaySound2D` "/Game/Music/Laser.Laser" 1.0 1.0 0.0 null null))

(fn `UserConstructionScript`
  (`parent.UserConstructionScript`))