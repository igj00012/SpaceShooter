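; Space shooter enemy generator that spawns random enemies on a looping timer while its live count is below the game mode's maximum.
; Each spawn picks a random SpawnPoint-tagged component and an enemy class, including a boss, limited by the game mode's type count.
; Each enemy's destroy event decrements the count and SpawnTime, though the running timer is never reset with the new interval.
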(event `self.ReceiveBeginPlay`
  (`KismetSystemLibrary.K2_SetTimerDelegate` (delegate `Spawn`) (`self.SpawnTime`) true)
  (bind _asss_game_mode (cast `/Game/SpaceShooter/SS_GameMode` (`GameplayStatics.GetGameMode`)))
  (set `self.m_GameMode` _asss_game_mode))

(event `Spawn`
  (bind _enemy_spawned (`self.SpawnEnemy`))
  (add `/Game/SpaceShooter/Enemies/BP_SS_EnemyBase.OnEnemyDestroy` _enemy_spawned (delegate `EnemyDestroyed`)))

(event `EnemyDestroyed`
  (set `self.EnemyCount` (- (`self.EnemyCount`) 1))
  (set `self.SpawnTime` (- (`self.SpawnTime`) 1.0)))

(fn `GetClassToSpawn`
  (params (type :type Integer))
  (returns (Class :type "/Game/SpaceShooter/Enemies/BP_SS_EnemyBase Class Reference"))
  (return (select `int` (`KismetMathLibrary.Clamp` type 0 (- (`/Game/SpaceShooter/SS_GameMode.EnemyTpes` (`self.m_GameMode`)) 1)) :`0` "/Game/SpaceShooter/Enemies/BP_SS_EnemyBase.BP_SS_EnemyBase_C" :`1` "/Game/SpaceShooter/Enemies/BP_SS_EnemyH.BP_SS_EnemyH_C" :`2` "/Game/SpaceShooter/Enemies/BP_SS_Enemy2FP.BP_SS_Enemy2FP_C" :`3` "/Game/SpaceShooter/Enemies/BP_SS_EnemyL.BP_SS_EnemyL_C" :`4` "/Game/SpaceShooter/Enemies/BP_SS_EnemyBoss.BP_SS_EnemyBoss_C" :!type "/Game/SpaceShooter/Enemies/BP_SS_EnemyBase Class Reference")))

(fn `SpawnEnemy`
  (returns (`Enemy Spawned` :type "/Game/SpaceShooter/Enemies/BP_SS_EnemyBase Object Reference"))
  (bind _returnvalue (`self.GetComponentsByTag` "/Script/Engine.SceneComponent" "SpawnPoint"))
  (bind _m_gamemode (`self.m_GameMode`))
  (if (< (`self.EnemyCount`) (`/Game/SpaceShooter/SS_GameMode.MaxEnemiesToSpawn` _m_gamemode))
    (bind _class (`self.GetClassToSpawn` (`KismetMathLibrary.RandomInteger` (`/Game/SpaceShooter/SS_GameMode.EnemyTpes` _m_gamemode))))
    (bind _returnvalue_2 (`|SpawnActorFromClass` _class (`SceneComponent.K2_GetComponentToWorld` (`|GetArrayItem` _returnvalue (`KismetMathLibrary.RandomInteger` (`KismetArrayLibrary.Array_Length` _returnvalue)))) "Undefined" "MultiplyWithRoot" null null))
    (set `self.EnemyCount` (+ (`self.EnemyCount`) 1))
    (return _returnvalue_2)))

(fn `UserConstructionScript`)